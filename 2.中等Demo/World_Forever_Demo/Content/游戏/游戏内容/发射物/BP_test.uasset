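; BP_test is a test projectile Blueprint that deals physical damage to enemies it touches.
; When its Sphere begins overlapping a BP-敌人模板 enemy, it calls 应用伤害物法 on its creator (创建者), passing the creator's attack power plus a flat bonus.
; It then sets its in-use flag (正在使用) to false rather than destroying itself.
; A debug print of damage and crit results is left unconnected.
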(event OnComponentBeginOverlap(Sphere)
  (params (OverlappedComponent :type Primitive%20Component%20Object%20Reference) (OtherActor :type Actor%20Object%20Reference) (OtherComp :type Primitive%20Component%20Object%20Reference) (OtherBodyIndex :type Integer) (bFromSweep :type Boolean) (SweepResult :type Hit%20Result%20Structure%20%28by%20ref%29))
  (bind _创建者 (Variables|Default|Get创建者))
  (bind _asbp_敌人模板 (Utilities|Casting|CastToBP-敌人模板 OtherActor))
  (bind (_实际造成物伤 _实际造成法伤 _是否触发暴击) (Default|应用伤害--物法 _创建者 _创建者 _asbp_敌人模板 (+ (.攻击力 (Utilities|Struct|BreakS-角色基础状态 (Variables|/Game/游戏/游戏内容/AC-角色对局状态.AC-角色对局状态_C|Get角色状态 (Variables|/Game/游戏/游戏内容/BP-总类.BP-总类_C|GetAC-角色对局状态 (Variables|Default|Get创建者))))) 1e+01) 0.0))
  (CallFunction|设置变量-正在使用 false))

(event EventBeginPlay
  (|CallParentFunction) ; 此节点被禁用，将不会被调用。\n从引脚连出引线来编译功能。
)

(event Collision|EventActorBeginOverlap
  (params (OtherActor :type Actor%20Object%20Reference))
  (|CallParentFunction OtherActor) ; 此节点被禁用，将不会被调用。\n从引脚连出引线来编译功能。
)

(event EventTick
  (params (DeltaSeconds :type Float%20%28single-precision%29))
  (|CallParentFunction DeltaSeconds) ; 此节点被禁用，将不会被调用。\n从引脚连出引线来编译功能。
)

(fn ConstructionScript
  (|CallParentFunction))