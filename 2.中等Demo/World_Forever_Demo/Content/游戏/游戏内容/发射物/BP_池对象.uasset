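; BP_池对象 is a pooled projectile that is toggled between active and dormant instead of being spawned and destroyed.
; It starts dormant, and its in-use setter switches collision, visibility and actor tick together.
; On activation it launches along its forward vector at travel distance divided by lifetime.
; A timer, cleared on every state change, returns it to the dormant state when that lifetime expires.
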(event Custom|将正在使用的放进池子里
  (CallFunction|设置变量-正在使用 false))

(event Custom|设置变量-正在使用
  (params (InUse :type Boolean))
  (bind _output_get (Variables|Default|Set正在使用 InUse))
  (Collision|SetActorEnableCollision _output_get)
  (Rendering|SetActorHiddenInGame (not _output_get))
  (Actor|Tick|SetActorTickEnabled _output_get)
  (Utilities|Time|ClearandInvalidateTimerbyHandle (Variables|Default|Get定时器柄))
  (if _output_get
    (bind _returnvalue (Utilities|Time|SetTimerbyEvent (delegate Custom|将正在使用的放进池子里) (Variables|Default|Get存活时间)))
    (Variables|Default|Set定时器柄 _returnvalue)
    (Variables|/Script/Engine.MovementComponent|SetVelocity (Variables|Default|GetProjectileMovement) (* (Transformation|GetActorForwardVector) (/ (Variables|Default|Get移动距离) (Variables|Default|Get存活时间))))))

(event EventBeginPlay
  (CallFunction|设置变量-正在使用 false))

(event Collision|EventActorBeginOverlap
  (params (OtherActor :type Actor%20Object%20Reference)))

(event EventTick
  (params (DeltaSeconds :type Float%20%28single-precision%29)))

(fn ConstructionScript)