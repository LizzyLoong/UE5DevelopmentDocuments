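; Object pool component, filed under projectiles, that pre-spawns reusable actors for its BP-角色模板 owner.
; On BeginPlay, 初始化池 spawns 池大小 instances of PooledActorClass at the owner's transform and marks them unused.
; 从池中生成 takes the first free actor, moves it, sets its lifetime and travel distance, then marks it in use.
; The pool never grows; an exhausted pool only prints a failure message.
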(event Custom|初始化池
  (bind _returnvalue (Components|GetOwner))
  (bind _asbp_角色模板 (Utilities|Casting|CastToBP-角色模板 _returnvalue))
  (for _index (range 0 (Variables|Default|Get池大小))
    (bind _returnvalue_2 (Game|SpawnActorfromClass (Variables|Default|GetPooledActorClass) (Transformation|GetActorTransform _asbp_角色模板) "Undefined" "MultiplyWithRoot" 0 0.5 0.0 _asbp_角色模板 0))
    (Utilities|Array|AddUnique (Variables|Default|GetPooledActor) _returnvalue_2)
    (Default|设置变量-正在使用 _returnvalue_2 false)))

(event EventBeginPlay
  (CallFunction|初始化池))

(event EventTick
  (params (DeltaSeconds :type Float%20%28single-precision%29)))

(fn 找到第一个可使用的Actor
  (for _array_element (Variables|Default|GetPooledActor)
    (if (not (Variables|/Game/游戏/游戏内容/发射物/BP_池对象.BP_池对象_C|Get正在使用 _array_element))
      (return _array_element))))

(fn 从池中生成
  (params (SpawnTransform :type Transform) (存活时间 :type Float%20%28double-precision%29) (移动距离 :type Float%20%28double-precision%29))
  (bind _pooledactor (CallFunction|找到第一个可使用的Actor))
  (Utilities|IsValid _pooledactor
    (:Is%20Valid
      (Transformation|SetActorTransform _pooledactor SpawnTransform)
      (Variables|/Game/游戏/游戏内容/发射物/BP_池对象.BP_池对象_C|Set移动距离 _pooledactor 移动距离)
      (Variables|/Game/游戏/游戏内容/发射物/BP_池对象.BP_池对象_C|Set存活时间 _pooledactor 存活时间)
      (Default|设置变量-正在使用 _pooledactor true)
      (return _pooledactor))
    (:Is%20Not%20Valid
      (Development|PrintText "从池中生成函数，生成失败" true true "(R=1.000000,G=0.000000,B=0.008680,A=1.000000)"))))